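; BP_Player_Fly is a player pawn that drifts constantly along world +X while accepting directional movement input.
; Each Tick calls ConstatntMove, which shifts the root one unit in X without sweep, so drift speed depends on frame rate despite the stored DeltaTime.
; The MoveUp and MOveRight axes feed AddMovementInput along the actor's forward and right vectors, so MoveUp moves forward rather than vertically.
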(event Custom|ConstatntMove
  (bind _returnvalue (Transformation|GetActorLocation))
  ;[1 1 1] ConstatntMove
  (Transformation|SetWorldLocation (Variables|Default|GetDefaultSceneRoot) (Math|Vector|MakeVector (+ (.x _returnvalue) 1.0) (.y _returnvalue) (.z _returnvalue)) false false))

(event EventTick
  (params (DeltaSeconds :type Float%20%28single-precision%29))
  (Variables|Default|SetDeltaTime DeltaSeconds)
  (CallFunction|ConstatntMove))

(event Input|AxisEvents|InputAxisMoveUp
  (params (AxisValue :type Float%20%28single-precision%29))
  ;[1 1 1] Movement
  (Pawn|Input|AddMovementInput (Transformation|GetActorForwardVector) AxisValue false))

(event Input|AxisEvents|InputAxisMOveRight
  (params (AxisValue :type Float%20%28single-precision%29))
  ;[1 1 1] Movement
  (Pawn|Input|AddMovementInput (Transformation|GetActorRightVector) AxisValue false))

(fn ConstructionScript)