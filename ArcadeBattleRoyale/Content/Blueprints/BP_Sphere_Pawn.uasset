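; BP_Sphere_Pawn is a pawn whose Sphere component is moved by directional step functions.
; MoveUp, MoveDown, MoveRight and MoveLeft offset its world location along X or Y by Speed, while ConstantMove advances it along +X by ConstantSpeed.
; Each teleports without sweep or delta-time scaling, so movement ignores collision.
; The event graph is empty, so these functions are not called within this Blueprint.
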(event EventBeginPlay)

(event Collision|EventActorBeginOverlap
  (params (OtherActor :type Actor%20Object%20Reference)))

(event EventTick
  (params (DeltaSeconds :type Float%20%28single-precision%29)))

(fn ConstructionScript)

(fn MoveUp
  (bind _sphere (Variables|Default|GetSphere))
  (bind _returnvalue (Transformation|GetWorldLocation _sphere))
  (Transformation|SetWorldLocation _sphere (Math|Vector|MakeVector (+ (.x _returnvalue) (Variables|Default|GetSpeed)) (.y _returnvalue) (.z _returnvalue)) false false))

(fn MoveRight
  (bind _sphere (Variables|Default|GetSphere))
  (bind _returnvalue (Transformation|GetWorldLocation _sphere))
  (Transformation|SetWorldLocation _sphere (Math|Vector|MakeVector (.x _returnvalue) (+ (.y _returnvalue) (Variables|Default|GetSpeed)) (.z _returnvalue)) false false))

(fn MoveLeft
  (bind _sphere (Variables|Default|GetSphere))
  (bind _returnvalue (Transformation|GetWorldLocation _sphere))
  (Transformation|SetWorldLocation _sphere (Math|Vector|MakeVector (.x _returnvalue) (- (.y _returnvalue) (Variables|Default|GetSpeed)) (.z _returnvalue)) false false))

(fn MoveDown
  (bind _sphere (Variables|Default|GetSphere))
  (bind _returnvalue (Transformation|GetWorldLocation _sphere))
  (Transformation|SetWorldLocation _sphere (Math|Vector|MakeVector (- (.x _returnvalue) (Variables|Default|GetSpeed)) (.y _returnvalue) (.z _returnvalue)) false false))

(fn ConstantMove
  (bind _sphere (Variables|Default|GetSphere))
  (bind _returnvalue (Transformation|GetWorldLocation _sphere))
  (Transformation|SetWorldLocation _sphere (Math|Vector|MakeVector (+ (.x _returnvalue) (Variables|Default|GetConstantSpeed)) (.y _returnvalue) (.z _returnvalue)) false false))