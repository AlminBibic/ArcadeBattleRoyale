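; BP_GameMode is a game mode that spawns players as sphere pawns and can point their views at a shared camera.
; For each new player, the authority spawns a BP_Sphere_Pawn at a player start, possesses it and stores the controller in an array.
; FindCamera runs only on BeginPlay, switching every stored controller to the first BP_Camera if the array length equals WaitForPlayerNum.
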(event EventHandleStartingNewPlayer
  (params (NewPlayer :type Player%20Controller%20Object%20Reference))
  (Networking|SwitchHasAuthority
    (:Authority
      (bind _returnvalue (Game|SpawnActorfromClass "/Game/Blueprints/BP_Sphere_Pawn.BP_Sphere_Pawn_C" (Transformation|GetActorTransform (Class|GameModeBase|FindPlayerStart)) "AdjustIfPossibleButAlwaysSpawn" NewPlayer 0))
      (Pawn|Possess NewPlayer _returnvalue)
      (Development|PrintString (Utilities|String|Append "Player connected: " (Utilities|GetDisplayName NewPlayer)))
      (Utilities|Array|Add (Variables|Default|GetPlayerController) NewPlayer))))

(event EventBeginPlay
  (CallFunction|FindCamera))

(fn ConstructionScript)

(fn FindCamera
  (if (== (Utilities|Array|Length (Variables|Default|GetPlayerController)) (Variables|Default|GetWaitForPlayerNum))
    (for _array_element (Variables|Default|GetPlayerController)
      (bind _outactors (Actor|GetAllActorsOfClass "/Game/Blueprints/BP_Camera.BP_Camera_C"))
      (Game|Player|SetViewTargetwithBlend _array_element (Utilities|Array|Get(acopy) _outactors) 0.0 "VTBlend_Linear" 0.0 false))))