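; Player controller that forwards movement input to the controlled BP_Sphere_Pawn through Server-prefixed events.
; Each tick it checks the signs of the up and right axes to call the matching directional move on the pawn, and also triggers its constant move regardless of input.
; On BeginPlay it asks BP_GameMode to find the camera.
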(event Custom|ServerMoveUp
  (bind _asbp_sphere_pawn (Utilities|Casting|CastToBP_Sphere_Pawn (Pawn|GetControlledPawn)))
  (Default|MoveUp _asbp_sphere_pawn))

(event Custom|ServerFindCamera
  (bind _asbp_game_mode (Utilities|Casting|CastToBP_GameMode (Game|GetGameMode)))
  (Default|FindCamera _asbp_game_mode))

(event Custom|ServerMoveDown
  (bind _asbp_sphere_pawn (Utilities|Casting|CastToBP_Sphere_Pawn (Pawn|GetControlledPawn)))
  (Default|MoveDown _asbp_sphere_pawn))

(event Custom|ServerMoveRight
  (bind _asbp_sphere_pawn (Utilities|Casting|CastToBP_Sphere_Pawn (Pawn|GetControlledPawn)))
  (Default|MoveRight _asbp_sphere_pawn))

(event Custom|ServerMoveLeft
  (bind _asbp_sphere_pawn (Utilities|Casting|CastToBP_Sphere_Pawn (Pawn|GetControlledPawn)))
  (Default|MoveLeft _asbp_sphere_pawn))

(event Custom|ServerConstantMoveUp
  (bind _asbp_sphere_pawn (Utilities|Casting|CastToBP_Sphere_Pawn (Pawn|GetControlledPawn)))
  (Default|ConstantMove _asbp_sphere_pawn))

(event EventBeginPlay
  (CallFunction|ServerFindCamera))

(event EventTick
  (params (DeltaSeconds :type Float%20%28single-precision%29))
  (bind _returnvalue (Input|AxisValues|GetMoveUp))
  (bind _returnvalue_2 (Input|AxisValues|GetMOveRight))
  (Utilities|FlowControl|Sequence
    (:then_0
      (if (> _returnvalue 0.0)
        (CallFunction|ServerMoveUp)))
    (:then_1
      (if (< _returnvalue 0.0)
        (CallFunction|ServerMoveDown)))
    (:then_2
      (if (> _returnvalue_2 0.0)
        (CallFunction|ServerMoveRight)))
    (:then_3
      (if (< _returnvalue_2 0.0)
        (CallFunction|ServerMoveLeft)))
    (:then_4
      (CallFunction|ServerConstantMoveUp))))

(fn ConstructionScript)